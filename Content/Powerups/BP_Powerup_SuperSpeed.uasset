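; BP_Powerup_SuperSpeed is a powerup that temporarily doubles the movement speed of the player it is activated for.
; OnActivated stores that player and sets the CharacterMovementComponent's MaxWalkSpeed to twice its GetMaxSpeed value.
; OnExpired sets MaxWalkSpeed to half the current GetMaxSpeed value if the stored player is still valid, then calls the parent's expiry logic.
; The change is relative, with no original speed saved.
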(event `self.OnActivated`
  (params (ActiveFor :type "Actor Object Reference"))
  (bind _returnvalue (`self.GetComponentByClass` ActiveFor "/Script/Engine.CharacterMovementComponent"))
  (set `self.ActiveForPlayer` ActiveFor)
  (set `CharacterMovementComponent.MaxWalkSpeed` (* 2 (`MovementComponent.GetMaxSpeed` _returnvalue)) _returnvalue))

(event `self.OnExpired`
  (bind _activeforplayer (`self.ActiveForPlayer`))
  (bind _returnvalue (`self.GetComponentByClass` _activeforplayer "/Script/Engine.CharacterMovementComponent"))
  (`/Engine/EditorBlueprintResources/StandardMacros.IsValid` _activeforplayer
    (:`Is Valid`
      (set `CharacterMovementComponent.MaxWalkSpeed` (/ (`MovementComponent.GetMaxSpeed` _returnvalue) 2.0) _returnvalue))
    (:`Is Not Valid`
      _))
  (`parent.OnExpired`))

(fn `UserConstructionScript`)